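; BP_Pawn is a player camera pawn with smoothed panning, stepped yaw rotation and spring arm zoom.
; Input only edits target values seeded at BeginPlay: axes pan along the actor's forward and right vectors or change clamped zoom, and key presses add fixed yaw steps.
; Tick interpolates actor location, rotation and arm length toward those targets, moving without sweep collision.
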(event `self.ReceiveBeginPlay`
  (set `self.Location_Value` (`self.K2_GetActorLocation`))
  (set `self.Zoom_Value` (`SpringArmComponent.TargetArmLength` (`self.SpringArm`)))
  (set `self.Rotation_Value` (`self.K2_GetActorRotation`)))

(event `InputAxis|InputAxis_Zoom`
  (params (AxisValue :type "Float (single-precision)"))
  (set `self.Zoom_Value` (`KismetMathLibrary.FClamp` (+ (`self.Zoom_Value`) (* AxisValue (`self.Zoom_Speed`))) (`self.Zoom_Min`) (`self.Zoom_Max`))))

(event `self.ReceiveTick`
  (params (DeltaSeconds :type "Float (single-precision)"))
  (bind _springarm (`self.SpringArm`))
  (set `SpringArmComponent.TargetArmLength` (`KismetMathLibrary.FInterpTo` (`SpringArmComponent.TargetArmLength` _springarm) (`self.Zoom_Value`) DeltaSeconds (`self.Zoom_Interp`)) _springarm)
  (`self.K2_SetActorLocation` (`KismetMathLibrary.VInterpTo` (`self.K2_GetActorLocation`) (`self.Location_Value`) DeltaSeconds (`self.Location_Interp`)))
  (`self.K2_SetActorRotation` (`KismetMathLibrary.RInterpTo` (`self.K2_GetActorRotation`) (`self.Rotation_Value`) DeltaSeconds (`self.Rotation_Interp`))))

(event `InputAxis|InputAxis_Vertical`
  (params (AxisValue :type "Float (single-precision)"))
  (set `self.Location_Value` (+ (`self.Location_Value`) (* (`self.GetActorForwardVector`) (* AxisValue (`self.Location_Speed`))))))

(event `InputAxis|InputAxis_Horizontal`
  (params (AxisValue :type "Float (single-precision)"))
  (set `self.Location_Value` (+ (`self.Location_Value`) (* (`self.GetActorRightVector`) (* AxisValue (`self.Location_Speed`))))))

(event `InputAction|InputAction_RotateLeft`
  (params (Key :type "Key Structure"))
  (:`Pressed`
    (set `self.Rotation_Value` (`KismetMathLibrary.ComposeRotators` (`self.Rotation_Value`) (`KismetMathLibrary.MakeRotator` 0.0 0.0 (- 0.0 (`self.Rotation_Speed`)))))))

(event `InputAction|InputAction_RotateRight`
  (params (Key :type "Key Structure"))
  (:`Pressed`
    (set `self.Rotation_Value` (`KismetMathLibrary.ComposeRotators` (`self.Rotation_Value`) (`KismetMathLibrary.MakeRotator` 0.0 0.0 (`self.Rotation_Speed`))))))

(fn `UserConstructionScript`)